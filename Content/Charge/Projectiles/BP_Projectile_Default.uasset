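; Default chargeable projectile Blueprint that grows with charge rate and reports a stun reaction tag for damage.
; Charge rate sets clamped actor scale and switches damage type to explosion above a threshold.
; On shooting, it offsets itself along its velocity by the scaled capsule radius; on hit, it fires a burst GameplayCue at the impact point.
; Construction tints the mesh through a dynamic emissive material.
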(event `self.ReceiveBeginPlay`
  (add `self.OnProjectileHit` (delegate `SpawnEmitter`))
  (set `self.DamageAmount` (`self.DamageAmount`)))

(event `SpawnEmitter` :!signature `self.OnProjectileHit`
  (params (HitResult :type "HitResult Structure (by ref)"))
  (bind (_bblockinghit _binitialoverlap _time _distance _location _impactpoint _normal _impactnormal) (`GameplayStatics.BreakHitResult` HitResult))
  (`GameplayCueFunctionLibrary.ExecuteGameplayCueOnActor` self (struct :`TagName` "GameplayCue.Projectile.Burst") (`AbilitySystemBlueprintLibrary.MakeGameplayCueParameters` 0.0 0.0 (struct) (struct) (struct) (struct) (struct) _impactpoint _impactnormal self null self)))

(event `self.OnChargeAmountSet`
  (bind _maxscalemultiplier (`self.MaxScaleMultiplier`))
  ;[1 1 1] Adjust actor scale by charge rate
  (`self.SetActorScale3D` (`KismetMathLibrary.Conv_DoubleToVector` (`KismetMathLibrary.FClamp` (* (`self.ChargeRate`) _maxscalemultiplier) 1.0 _maxscalemultiplier))))

(event `self.ShootProjectileToTarget`
  (bind _capsule (`self.Capsule`))
  (bind _projectilemovement (`self.ProjectileMovement`))
  (`parent.ShootProjectileToTarget`)
  (if (and (`KismetSystemLibrary.IsValid` _projectilemovement) (`KismetSystemLibrary.IsValid` _capsule))
    ;[1 1 1] Adjust spawn location considering projectile scale
    (`self.K2_AddActorWorldOffset` (* (`KismetMathLibrary.Normal` (`MovementComponent.Velocity` _projectilemovement)) (`CapsuleComponent.GetScaledCapsuleRadius` _capsule)))))

(fn `GetDamageAmount`
  (returns (ReturnValue :type "Float (single-precision)"))
  (return (`self.DamageAmount`)))

(fn `GetDamageReactionAbilityTag`
  (returns (ReturnValue :type "GameplayTagContainer Structure"))
  (return (struct :`GameplayTags` (struct :`(TagName` "Character.State.IsStunned")))))

(fn `GetDamageType`
  (returns (ReturnValue :type "DamageType Class Reference"))
  (if (>= (`self.ChargeRate`) 0.3)
    (return "/Script/Charge.DamageType_Explosion")
    (else
      (return "/Script/Engine.DamageType"))))

(fn `UserConstructionScript`
  (bind _returnvalue (`PrimitiveComponent.CreateDynamicMaterialInstance` (`self.StaticMesh`) 0 "/Engine/ArtTools/RenderToTexture/Materials/Debug/M_Emissive_Color.M_Emissive_Color" "MI_Emissive"))
  (`MaterialInstanceDynamic.SetVectorParameterValue` _returnvalue "Color" (`self.MaterialColor`)))