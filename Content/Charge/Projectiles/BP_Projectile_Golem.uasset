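; Charged projectile fired by the Golem enemy, which grows in place before launching at its attack target.
; Charge amount sets a clamped final scale, and a looping timer scales the actor up with collision off, then enables query collision and shoots.
; Aim leads the target using its velocity, and a high charge switches the damage type to explosion.
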(event `self.OnChargeAmountSet`
  (bind _maxscalemultiplier (`self.MaxScaleMultiplier`))
  (set `self.FinalScaleMultiplier` (`KismetMathLibrary.FClamp` (* (`self.ChargeRate`) _maxscalemultiplier) 1.0 _maxscalemultiplier)))

(event `self.ReceiveBeginPlay`
  (bind _instigator (`self.Instigator`))
  (`parent.ReceiveBeginPlay`)
  (`PrimitiveComponent.SetCollisionEnabled` (`self.Capsule`) "NoCollision")
  (if (`KismetSystemLibrary.IsValid` _instigator)
    (`self.K2_AddActorWorldOffset` (* (`self.GetActorForwardVector` _instigator) 80.0))
    ;[1 1 1] Start scale up animation
    (`MovementComponent.StopMovementImmediately` (`self.ProjectileMovement`))
    (set `self.ScaleUpLoopCount` 1)
    (bind _returnvalue (`KismetSystemLibrary.K2_SetTimerDelegate` (delegate `ScaleUpProjectile`) 0.05 true))
    (set `self.ScaleUpTimerHandle` _returnvalue)))

(event `ScaleUpProjectile`
  (`self.SetActorScale3D` (`KismetMathLibrary.Conv_DoubleToVector` (* (/ (`self.FinalScaleMultiplier`) 20.0) (`self.ScaleUpLoopCount`))))
  (bind _result (`/Engine/EditorBlueprintResources/StandardMacros.IncrementInt` (`self.ScaleUpLoopCount`))
    (:`  `
      (if (> _result 20)
        (`KismetSystemLibrary.K2_ClearAndInvalidateTimerHandle` (`self.ScaleUpTimerHandle`))
        (`PrimitiveComponent.SetCollisionEnabled` (`self.Capsule`) "QueryOnly")
        (`self.ShootProjectileToTarget`)))))

(event `self.ShootProjectileToTarget`
  (bind _ascpenemy_character (cast `CPEnemyCharacter` (`self.Instigator`)))
  (bind _attacktarget (`CPEnemyCharacter.AttackTarget` _ascpenemy_character))
  (if (`KismetSystemLibrary.IsValid` _attacktarget)
    (set `self.ProjectileTargetLocation` (+ (`self.K2_GetActorLocation` _attacktarget) (/ (`self.GetVelocity` _attacktarget) 3.0))))
  (`parent.ShootProjectileToTarget`))

(event `self.ReceiveEndPlay`
  (params (EndPlayReason :type "EEndPlayReason Enum" :default "Destroyed"))
  (bind _scaleuptimerhandle (`self.ScaleUpTimerHandle`))
  (if (`KismetSystemLibrary.K2_IsTimerActiveHandle` _scaleuptimerhandle)
    (`KismetSystemLibrary.K2_ClearAndInvalidateTimerHandle` _scaleuptimerhandle)))

(fn `GetDamageType`
  (returns (ReturnValue :type "DamageType Class Reference"))
  (if (>= (`self.ChargeRate`) 0.8)
    (return "/Script/Charge.DamageType_Explosion")
    (else
      (return "/Script/Engine.DamageType"))))

(fn `UserConstructionScript`)