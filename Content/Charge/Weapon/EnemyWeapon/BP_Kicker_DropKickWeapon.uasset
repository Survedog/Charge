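; BP_Kicker_DropKickWeapon is an enemy weapon that gives the Kicker a drop-kick combo attack.
; Starting the combo switches the owning character's movement to Flying, and ending the primary attack restores Walking, each before calling the parent logic.
; Overrides supply the drop-kick montage and an explosion damage type for the melee hit, with no projectile class.
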(event `self.StartComboAttack`
  (params (InChargeRate :type "Float (single-precision)"))
  (bind _cpcharacterowner (`self.CPCharacterOwner`))
  (if (`KismetSystemLibrary.IsValid` _cpcharacterowner)
    (`CharacterMovementComponent.SetMovementMode` (`Character.CharacterMovement` _cpcharacterowner) "MOVE_Flying" 0))
  (`parent.StartComboAttack` InChargeRate))

(event `self.EndPrimaryAttack`
  (bind _cpcharacterowner (`self.CPCharacterOwner`))
  (if (`KismetSystemLibrary.IsValid` _cpcharacterowner)
    (`CharacterMovementComponent.SetMovementMode` (`Character.CharacterMovement` _cpcharacterowner) "MOVE_Walking" 0))
  (`parent.EndPrimaryAttack`))

(fn `GetMeeleAttackDamageType`
  (returns (ReturnValue :type "DamageType Class Reference"))
  (return "/Script/Charge.DamageType_Explosion"))

(fn `GetPrimaryAttackMontage`
  (returns (ReturnValue :type "AnimMontage Object Reference"))
  (return "/Game/Charge/Animation/Enemy/Kicker/AM_Kicker_DropKick.AM_Kicker_DropKick"))

(fn `GetProjectileClass`
  (returns (ReturnValue :type "CPProjectileBase Class Reference"))
  (return null))