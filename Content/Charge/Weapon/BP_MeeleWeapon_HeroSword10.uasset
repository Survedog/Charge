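; Hero sword melee weapon Blueprint whose combo attack gains range with charge.
; On combo start it applies a gameplay effect to the owner, setting the range multiplier by SetByCaller from a linear ease of the current charge rate up to MaxAttackRange.
; Ending the primary attack removes that effect through its stored handle.
; Overrides also supply the sword montage, damage type and stunned damage-reaction tag.
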(event `self.StartComboAttack`
  (params (InChargeRate :type "Float (single-precision)"))
  (bind _returnvalue (`AbilitySystemBlueprintLibrary.GetAbilitySystemComponent` (`self.CPCharacterOwner`)))
  (`parent.StartComboAttack` InChargeRate)
  ;[1 1 1] Apply ExpandAttackRange Effect
  (bind _returnvalue_2 (`AbilitySystemBlueprintLibrary.AssignTagSetByCallerMagnitude` (`AbilitySystemComponent.MakeOutgoingSpec` _returnvalue "/Game/Charge/Blueprint/GE/WeaponSpecific/BPGE_HeroSword_Attack.BPGE_HeroSword_Attack_C" 0.0 (`AbilitySystemComponent.MakeEffectContext` _returnvalue)) (struct :`TagName` "Character.Stat.MeeleAttackRangeMultiplier") (`|EaseFunction` "Linear" (`self.CurrentAttackChargeRate`) 1.0 (`self.MaxAttackRange`))))
  (bind _returnvalue_3 (`AbilitySystemComponent.BP_ApplyGameplayEffectSpecToSelf` _returnvalue _returnvalue_2))
  (set `self.ActiveHeroSwordAttackEffect` _returnvalue_3))

(event `self.EndPrimaryAttack`
  (bind _returnvalue (`AbilitySystemBlueprintLibrary.GetAbilitySystemComponent` (`self.CPCharacterOwner`)))
  ;[1 1 1] Remove ExpandAttackRange Effect
  (if (`KismetSystemLibrary.IsValid` _returnvalue)
    (`AbilitySystemComponent.RemoveActiveGameplayEffect` _returnvalue (`self.ActiveHeroSwordAttackEffect`) -1)
    (set `self.ActiveHeroSwordAttackEffect` (struct))
    (`parent.EndPrimaryAttack`)))

(fn `GetDamageReactionAbilityTag`
  (returns (ReturnValue :type "GameplayTagContainer Structure"))
  (return (struct :`GameplayTags` (struct :`(TagName` "Character.State.IsStunned")))))

(fn `GetMeeleAttackDamageType`
  (returns (ReturnValue :type "DamageType Class Reference"))
  (return "/Script/Engine.DamageType"))

(fn `GetPrimaryAttackMontage`
  (returns (ReturnValue :type "AnimMontage Object Reference"))
  (return "/Game/Charge/Animation/Player/Sword/AM_Player_Attack_Sword.AM_Player_Attack_Sword"))