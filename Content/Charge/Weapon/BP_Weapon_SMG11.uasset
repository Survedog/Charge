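; SMG11 weapon Blueprint that fires SMG projectiles as a primary attack and supplies timing for a charge-scaled attack.
; PrimaryAttack spawns projectiles through SpawnProjectileOnAll, while StartComboAttack defers to the parent.
; The fire montage switches between ironsight and hip rifle animations based on the owner's Aim gameplay tag.
; Charge rate sets attack period and duration, with higher charge shortening the period to a floor and lengthening the duration to a cap.
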(event `self.StartComboAttack`
  (params (InChargeRate :type "Float (single-precision)"))
  (`parent.StartComboAttack` InChargeRate))

(event `self.PrimaryAttack`
  (params (InComboCount :type Integer))
  (`self.SpawnProjectileOnAll`))

(fn `GetAttackDuration`
  (params (InChargeRate :type "Float (single-precision)"))
  (returns (ReturnValue :type "Float (single-precision)"))
  (return (`KismetMathLibrary.FMin` (* InChargeRate 3.0) 3.0)))

(fn `GetAttackPeriod`
  (params (InChargeRate :type "Float (single-precision)"))
  (returns (ReturnValue :type "Float (single-precision)"))
  (return (`KismetMathLibrary.FMax` (/ 0.05 InChargeRate) 0.1)))

(fn `GetPrimaryAttackMontage`
  (returns (ReturnValue :type "AnimMontage Object Reference"))
  (bind _cpcharacterowner (`self.CPCharacterOwner`))
  (if (`KismetSystemLibrary.IsValid` _cpcharacterowner)
    (if (`GameplayTagAssetInterface.HasMatchingGameplayTag` (`AbilitySystemBlueprintLibrary.GetAbilitySystemComponent` _cpcharacterowner) (struct :`TagName` "Character.Action.Aim"))
      (return "/Game/Charge/Animation/Player/Rifle/AM_Player_Fire_Ironsight_Rifle.AM_Player_Fire_Ironsight_Rifle")
      (else
        (return "/Game/Charge/Animation/Player/Rifle/AM_Player_Fire_Hip_Rifle.AM_Player_Fire_Hip_Rifle")))))

(fn `GetProjectileClass`
  (returns (ReturnValue :type "CPProjectileBase Class Reference"))
  (return "/Game/Charge/Blueprint/Projectiles/BP_Projectile_SMG.BP_Projectile_SMG_C"))