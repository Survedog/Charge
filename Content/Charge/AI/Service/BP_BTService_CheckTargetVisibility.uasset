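; Behavior tree service that updates whether the AI's target is visible.
; Each tick it sphere traces from the controlled pawn's eye viewpoint to the blackboard target's location, ignoring both actors.
; It writes the visibility blackboard bool as true when nothing blocks the trace, and leaves it untouched when the target is invalid.
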(event `self.ReceiveTickAI`
  (params (OwnerController :type "AIController Object Reference") (ControlledPawn :type "Pawn Object Reference") (DeltaSeconds :type "Float (single-precision)"))
  (bind _returnvalue (`BTFunctionLibrary.GetBlackboardValueAsActor` (`self.BBTarget`)))
  (if (`KismetSystemLibrary.IsValid` _returnvalue)
    (bind (_outhit _returnvalue_2) (`KismetSystemLibrary.SphereTraceSingle` (`Actor.GetActorEyesViewPoint` ControlledPawn) (`Actor.K2_GetActorLocation` _returnvalue) (`self.TraceSphereRadius`) "TraceTypeQuery3" false (`|MakeArray` _returnvalue ControlledPawn :!type "Actor Object Reference") "None" true (struct :`R` 1.0 :`A` 1.0) (struct :`G` 1.0 :`A` 1.0) 0.5))
    (`BTFunctionLibrary.SetBlackboardValueAsBool` (`self.BBIsTargetVisible`) (not _returnvalue_2))))