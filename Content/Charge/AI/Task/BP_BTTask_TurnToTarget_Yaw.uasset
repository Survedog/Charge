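; Behavior tree task that turns the AI-controlled pawn on the yaw axis to face the blackboard's TargetActor.
; On AI tick it compares the look-at yaw with the pawn's yaw and, outside YawDiffTolerance, adds the whole difference as world rotation.
; The turn is an instant snap without interpolation or angle normalization, and the task then finishes successfully on that same tick.
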(event `self.ReceiveTickAI`
  (params (OwnerController :type "AIController Object Reference") (ControlledPawn :type "Pawn Object Reference") (DeltaSeconds :type "Float (single-precision)"))
  (bind (_returnvalue_roll _returnvalue_pitch _returnvalue_yaw) (`KismetMathLibrary.BreakRotator` (`Actor.K2_GetActorRotation` ControlledPawn)))
  (bind (_returnvalue_roll_2 _returnvalue_pitch_2 _returnvalue_yaw_2) (`KismetMathLibrary.BreakRotator` (`KismetMathLibrary.FindLookAtRotation` (`Actor.K2_GetActorLocation` ControlledPawn) (`Actor.K2_GetActorLocation` (`BTFunctionLibrary.GetBlackboardValueAsActor` (`self.TargetActor`))))))
  (bind _returnvalue (- _returnvalue_yaw_2 _returnvalue_yaw))
  (if (not (`KismetMathLibrary.NearlyEqual_FloatFloat` _returnvalue 0.0 (`self.YawDiffTolerance`)))
    (`Actor.K2_AddActorWorldRotation` ControlledPawn (`KismetMathLibrary.MakeRotator` 0.0 0.0 _returnvalue) false false))
  (`self.FinishExecute` true))