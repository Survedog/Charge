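; Behavior tree task that moves the AI pawn to a random reachable navmesh point within MoveRadius of the blackboard Target actor.
; It passes the point to AIMoveTo, succeeds after a short delay on arrival, fails if the move fails, and stops movement on abort.
; A debug print evaluates its own random point, so the printed location can differ from the actual destination.
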(event `self.ReceiveExecuteAI`
  (params (OwnerController :type "AIController Object Reference") (ControlledPawn :type "Pawn Object Reference"))
  (bind _returnvalue (`GameplayStatics.GetActorOfClass` "/Script/NavigationSystem.NavigationData"))
  (bind _randomlocation (`NavigationSystemV1.K2_GetRandomReachablePointInRadius` (`NavigationSystemV1.GetNavigationSystem`) (`Actor.K2_GetActorLocation` (`BTFunctionLibrary.GetBlackboardValueAsActor` (`self.Target`))) (`self.MoveRadius`) _returnvalue null))
  (`KismetSystemLibrary.PrintString` (`KismetStringLibrary.Conv_VectorToString` _randomlocation))
  (`|AIMoveTo` OwnerController ControlledPawn _randomlocation null (`self.Acceptance Radius`)
    (:`OnSuccess`
      (`KismetSystemLibrary.Delay` 0.5)
      (`self.FinishExecute` true))
    (:`OnFail`
      (`self.FinishExecute` false))))

(event `self.ReceiveAbortAI`
  (params (OwnerController :type "AIController Object Reference") (ControlledPawn :type "Pawn Object Reference"))
  (`Controller.StopMovement` OwnerController)
  (`self.FinishAbort`))