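; Behavior tree task that switches an AI-controlled CPEnemyCharacter to another weapon in its inventory.
; On execute it casts the controlled pawn and checks that the configured weapon index exists in the weapon component's inventory.
; It then calls SwapCurrentWeapon with the enemy's ability system component, flagged as not a new weapon, and succeeds.
; A failed cast or invalid index finishes the task as failed.
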(event `self.ReceiveExecuteAI`
  (params (OwnerController :type "AIController Object Reference") (ControlledPawn :type "Pawn Object Reference"))
  (bind _ascpenemy_character (cast `CPEnemyCharacter` ControlledPawn)
    (:`then`
      (if (`KismetArrayLibrary.Array_IsValidIndex` (`CharacterWeaponComponent.WeaponInventory` (`CPCharacterBase.WeaponComp` _ascpenemy_character)) (`self.WeaponIndexToSwap`))
        (`CharacterWeaponComponent.SwapCurrentWeapon` (`CPCharacterBase.WeaponComp` _ascpenemy_character) (`self.WeaponIndexToSwap`) (`AbilitySystemBlueprintLibrary.GetAbilitySystemComponent` _ascpenemy_character) false)
        (`self.FinishExecute` true)
        (else
          (`self.FinishExecute` false :!label _label))))
    (:`CastFailed`
      (goto _label))))